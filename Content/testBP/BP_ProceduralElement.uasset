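; Modular procedural building-block actor that switches meshes for its connection points and optional areas.
; Construction script discovers connector arrows and optional areas from the component hierarchy, matching state children by display-name substrings.
; Boolean arrays, matched by index, toggle mesh visibility and collision between each pair on construction and BeginPlay.
; Helpers look up connectors by name and spawn, set up or destroy a random decoration Blueprint, though nothing here calls them.
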(event `self.ReceiveBeginPlay`
  (`self.UpdateConnections`)
  (`self.UpdateOptionalAreas`))

(fn `ActivateOptionalArea`
  (params (OptionalArea :type "/Game/testBP/Struct_OptionalArea Structure"))
  (bind (_optionalarea _activescenecomponentref _notactivescenecomponentref) (break `/Game/testBP/Struct_OptionalArea` OptionalArea))
  (`self.SetupSceneRefComponents` _activescenecomponentref _notactivescenecomponentref))

(fn `AdditionalSetup`
  (if (`KismetSystemLibrary.IsValid` (`self.DecorationBlueprint`))
    (`self.AdditionalSetup` (`self.DecorationBlueprint`))))

(fn `BuildConnectorsArray`
  (locals (NewLocalVar_0 :type Boolean) (IsConnectedSceneComponentRef :type "SceneComponent Object Reference") (IsNotConnectedSceneComponentReference :type "SceneComponent Object Reference"))
  (`KismetArrayLibrary.Array_Clear` (`self.Connectors`))
  (for _array_element (`SceneComponent.GetChildrenComponents` (`self.Connections`) false)
    (bind _asarrow_component (cast `ArrowComponent` _array_element))
    (for _array_element_2 (`SceneComponent.GetChildrenComponents` _asarrow_component false)
      (bind _returnvalue (`KismetSystemLibrary.GetDisplayName` _array_element_2))
      (if (`KismetStringLibrary.Contains` _returnvalue "isconnected")
        (set `local.IsConnectedSceneComponentRef` _array_element_2))
      (if (`KismetStringLibrary.Contains` _returnvalue "isnotconnected")
        (set `local.IsNotConnectedSceneComponentReference` _array_element_2)))
    (`KismetArrayLibrary.Array_Add` (`self.Connectors`) (make `/Game/testBP/Struct_Connection` _asarrow_component (`local.IsConnectedSceneComponentRef`) (`local.IsNotConnectedSceneComponentReference`)))))

(fn `BuildOptionalAreasArray`
  (locals (ActiveSceneComponentRef :type "SceneComponent Object Reference") (NotActiveSceneComponentRef :type "SceneComponent Object Reference"))
  (`KismetArrayLibrary.Array_Clear` (`self.OptionalAreas`))
  (for _array_element (`SceneComponent.GetChildrenComponents` (`self.Optional_Areas`) false)
    (for _array_element_2 (`SceneComponent.GetChildrenComponents` _array_element false)
      (bind _returnvalue (`KismetSystemLibrary.GetDisplayName` _array_element_2))
      (if (`KismetStringLibrary.Contains` _returnvalue "isactive")
        (set `local.ActiveSceneComponentRef` _array_element_2)
        (elif (`KismetStringLibrary.Contains` _returnvalue "isnotactive")
          (set `local.NotActiveSceneComponentRef` _array_element_2))))
    (`KismetArrayLibrary.Array_Add` (`self.OptionalAreas`) (make `/Game/testBP/Struct_OptionalArea` _array_element (`local.ActiveSceneComponentRef`) (`local.NotActiveSceneComponentRef`)))))

(fn `ClearDecorationBlueprint`
  (if (`KismetSystemLibrary.IsValid` (`self.DecorationBlueprint`))
    (`self.K2_DestroyActor` (`self.DecorationBlueprint`))))

(fn `DeactivateOptionalArea`
  (params (OptionalArea :type "/Game/testBP/Struct_OptionalArea Structure"))
  (bind (_optionalarea _activescenecomponentref _notactivescenecomponentref) (break `/Game/testBP/Struct_OptionalArea` OptionalArea))
  (`self.SetupSceneRefComponents` _notactivescenecomponentref _activescenecomponentref))

(fn `DisableConnection`
  (params (Connection :type "/Game/testBP/Struct_Connection Structure (by ref)"))
  (locals (ConnectedRef :type "SceneComponent Object Reference") (NotConnectedRef :type "SceneComponent Object Reference"))
  (bind (_connectionpoint _connectedscenecomponentref _notconnectedscenecomponentref) (break `/Game/testBP/Struct_Connection` Connection))
  (`self.SetupSceneRefComponents` _notconnectedscenecomponentref _connectedscenecomponentref))

(fn `DisableMeshComponents`
  (params (SceneComponent :type "SceneComponent Object Reference"))
  (if (`KismetSystemLibrary.IsValid` SceneComponent)
    (for _array_element (`SceneComponent.GetChildrenComponents` SceneComponent false)
      (bind _asstatic_mesh_component (cast `StaticMeshComponent` _array_element))
      (`SceneComponent.SetVisibility` _asstatic_mesh_component false false)
      (`PrimitiveComponent.SetCollisionEnabled` _asstatic_mesh_component "NoCollision"))
    (else
      (`KismetSystemLibrary.PrintString` "Hello"))))

(fn `EnableConnection`
  (params (Connection :type "/Game/testBP/Struct_Connection Structure (by ref)"))
  (locals (ConnectedRef :type "SceneComponent Object Reference") (NotConnectedRef :type "SceneComponent Object Reference"))
  (bind (_connectionpoint _connectedscenecomponentref _notconnectedscenecomponentref) (break `/Game/testBP/Struct_Connection` Connection))
  (`self.SetupSceneRefComponents` _connectedscenecomponentref _notconnectedscenecomponentref))

(fn `EnableMeshComponents`
  (params (SceneComponent :type "SceneComponent Object Reference"))
  (if (`KismetSystemLibrary.IsValid` SceneComponent)
    (for _array_element (`SceneComponent.GetChildrenComponents` SceneComponent false)
      (bind _asstatic_mesh_component (cast `StaticMeshComponent` _array_element))
      (`SceneComponent.SetVisibility` _asstatic_mesh_component true false)
      (`PrimitiveComponent.SetCollisionEnabled` _asstatic_mesh_component "QueryAndPhysics"))))

(fn `GetConnector`
  (params (ConnectionName :type String))
  (returns (Connection :type "/Game/testBP/Struct_Connection Structure"))
  (locals (Connector :type "/Game/testBP/Struct_Connection Structure"))
  (for _array_element (`self.Connectors`)
    (if (`KismetStringLibrary.Contains` (`KismetSystemLibrary.GetDisplayName` (`.ConnectionPoint_9_1000F93B4634153801B2E9BB592C0EA2` (break `/Game/testBP/Struct_Connection` _array_element))) ConnectionName true)
      (set `local.Connector` _array_element)
      (break)))
  (return (`local.Connector`)))

(fn `SetupSceneRefComponents`
  (params (ComponentToEnable :type "SceneComponent Object Reference") (ComponentToDisable :type "SceneComponent Object Reference"))
  (`self.EnableMeshComponents` ComponentToEnable)
  (`self.DisableMeshComponents` ComponentToDisable))

(fn `SpawnDecorationBlueprint`
  (bind _returnvalue (`|SpawnActorFromClass` (`|GetArrayItem` (`self.DecorationBlueprints`) (`KismetMathLibrary.RandomInteger` (`KismetArrayLibrary.Array_Length` (`self.DecorationBlueprints`)))) (`self.GetTransform` self) "Undefined" "OverrideRootScale" null null))
  (if (`KismetSystemLibrary.IsValid` _returnvalue)
    (set `self.DecorationBlueprint` _returnvalue)))

(fn `UpdateConnections`
  (bind _connectors (`self.Connectors`))
  (for (_array_element _array_index) (`self.ActiveConnections`)
    (if (< _array_index (`KismetArrayLibrary.Array_Length` _connectors))
      (if _array_element
        (bind _output (`|GetArrayItem` _connectors _array_index))
        (`self.EnableConnection` _output)
        (else
          (`self.DisableConnection` _output))))))

(fn `UpdateOptionalAreas`
  (bind _optionalareas (`self.OptionalAreas`))
  (for (_array_element _array_index) (`self.ActiveOptionalAreas`)
    (if (< _array_index (`KismetArrayLibrary.Array_Length` _optionalareas))
      (if _array_element
        (bind _output (`|GetArrayItem` _optionalareas _array_index))
        (`self.ActivateOptionalArea` _output)
        (else
          (`self.DeactivateOptionalArea` _output))))))

(fn `UserConstructionScript`
  (`self.BuildConnectorsArray`)
  (`self.BuildOptionalAreasArray`)
  (`self.UpdateConnections`)
  (`self.UpdateOptionalAreas`))