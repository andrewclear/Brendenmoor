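; Procedural room generator that builds a random connected layout on BeginPlay, then rebuilds navigation via console command.
; AttachRoom recursively spawns random room Blueprints at randomly enabled connectors until the room cap is passed, disabling the rest.
; SpawnElement destroys rooms whose tagged boxes overlap others, and marks rooms spawned below the minimum count to attempt at least one connection.
; Generate clears and restarts the whole layout whenever it ends below the minimum.
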(event `self.ReceiveBeginPlay`
  (`self.Generate`)
  (`self.SetupNavMesh`))

(fn `AttachRoom`
  (params (newRoom :type "/Game/testBP/BP_ProceduralElement Object Reference"))
  (locals (hasConnectedToAnotherElement :type Boolean))
  (bind _connectors (`/Game/testBP/BP_ProceduralElement.Connectors` newRoom))
  (bind _output (`|GetArrayItem` _connectors (`KismetMathLibrary.RandomInteger` (`KismetArrayLibrary.Array_Length` _connectors))))
  (if (`KismetSystemLibrary.IsValid` newRoom)
    (for _array_element (`/Game/testBP/BP_ProceduralElement.Connectors` newRoom)
      (bind _allroomswerecreated (`self.CheckIfAllRoomsWereCreated` :!label _label))
      (if _allroomswerecreated
        (`/Game/testBP/BP_ProceduralElement.DisableConnection` newRoom _array_element :!label _label_2)
        (elif (== (`KismetMathLibrary.RandomInteger` 2) 1)
          (`/Game/testBP/BP_ProceduralElement.EnableConnection` newRoom _array_element)
          (bind (_newroom _spawnfailed) (`self.SpawnElement` (`SceneComponent.K2_GetComponentToWorld` (`.ConnectionPoint_9_1000F93B4634153801B2E9BB592C0EA2` (break `/Game/testBP/Struct_Connection` _array_element)))))
          (if _spawnfailed
            (goto _label)
            (else
              (`self.AttachRoom` _newroom)
              (set `local.hasConnectedToAnotherElement` true)))
          (else
            (goto _label_2)))))
    (if (`/Game/testBP/BP_ProceduralElement.mustConnectOnce` newRoom)
      (if (`local.hasConnectedToAnotherElement`)
        (`/Game/testBP/BP_ProceduralElement.AdditionalSetup` newRoom)
        (else
          (`/Game/testBP/BP_ProceduralElement.EnableConnection` newRoom _output)
          (bind (_newroom_2 _spawnfailed_2) (`self.SpawnElement` (`SceneComponent.K2_GetComponentToWorld` (`.ConnectionPoint_9_1000F93B4634153801B2E9BB592C0EA2` (break `/Game/testBP/Struct_Connection` _output)))))
          (if _spawnfailed_2
            (`/Game/testBP/BP_ProceduralElement.DisableConnection` newRoom _output)
            (else
              (`self.AttachRoom` _newroom_2)
              (`/Game/testBP/BP_ProceduralElement.AdditionalSetup` newRoom)))))
      (else
        (`/Game/testBP/BP_ProceduralElement.AdditionalSetup` newRoom)))
    (else
      (`KismetSystemLibrary.PrintString` "newRoomNotValid"))))

(fn `CheckIfAllRoomsWereCreated`
  (returns (allRoomsWereCreated :type Boolean))
  (return (< (`self.NumberOfMainRooms`) (`KismetArrayLibrary.Array_Length` (`self.MainElementObjects`)))))

(fn `ClearAllElements`
  (for _array_element (`self.MainElementObjects`)
    (`/Game/testBP/BP_ProceduralElement.ClearDecorationBlueprint` _array_element)
    (`self.K2_DestroyActor` _array_element))
  (`KismetArrayLibrary.Array_Clear` (`self.MainElementObjects`)))

(fn `Generate`
  (locals (SpawnPoint :type "Transform Structure"))
  (bind _returnvalue (`KismetArrayLibrary.Array_Length` (`self.MainElementObjects`)))
  (`self.ClearAllElements` :!label _label)
  (bind (_newroom _spawnfailed) (`self.SpawnElement` (`local.SpawnPoint`) true))
  (if _spawnfailed
    (goto _label)
    (else
      (`self.AttachRoom` _newroom)
      (`KismetSystemLibrary.PrintString` (`KismetStringLibrary.BuildString_Int` "Number of rooms created = " "" _returnvalue) true true (struct :`G` 0.66 :`B` 1.0 :`A` 1.0) 20.0)
      (if (< _returnvalue (`self.MinNumberOfRooms`))
        (goto _label)))))

(fn `SetupNavMesh`
  (`KismetSystemLibrary.ExecuteConsoleCommand` "RebuildNavigation" null))

(fn `SpawnElement`
  (params (SpawnTransform :type "Transform Structure") (IsFirstRoom :type Boolean :default false))
  (returns (newRoom :type "/Game/testBP/BP_ProceduralElement Object Reference") (spawnFailed :type Boolean))
  (locals (spawnedRoom :type "/Game/testBP/BP_ProceduralElement Object Reference") (isOverlapping :type Boolean) (OverlapTag :type Name :default "OverlapDetector") (failedToSpawn :type Boolean))
  (bind _returnvalue (`|SpawnActorFromClass` (`|GetArrayItem` (`self.MainElementsBlueprints`) (`KismetMathLibrary.RandomInteger` (`KismetArrayLibrary.Array_Length` (`self.MainElementsBlueprints`)))) SpawnTransform "Undefined" "OverrideRootScale" null null))
  (if (`KismetSystemLibrary.IsValid` _returnvalue)
    (for _array_element (`self.GetOverlappingComponents` _returnvalue)
      (bind _asbox_collision (cast `BoxComponent` _array_element))
      (if (`KismetArrayLibrary.Array_Contains` (`ActorComponent.ComponentTags` _asbox_collision) (`local.OverlapTag`))
        (if (not (== (`ActorComponent.GetOwner` _asbox_collision) _returnvalue))
          (set `local.isOverlapping` true)
          (break))))
    (if (`local.isOverlapping`)
      (set `local.spawnedRoom` null :!label _label)
      (`self.K2_DestroyActor` _returnvalue)
      (set `local.failedToSpawn` true)
      (else
        (bind _output_get (set `local.spawnedRoom` _returnvalue))
        (`/Game/testBP/BP_ProceduralElement.SpawnDecorationBlueprint` _output_get)
        (if IsFirstRoom
          (`/Game/testBP/BP_ProceduralElement.AddStartingRoomBlocker` (`local.spawnedRoom`))
          (elif (< (`KismetArrayLibrary.Array_Length` (`self.MainElementObjects`)) (`self.MinNumberOfRooms`))
            (set `/Game/testBP/BP_ProceduralElement.mustConnectOnce` true (`local.spawnedRoom`))))
        (`KismetArrayLibrary.Array_Add` (`self.MainElementObjects`) (`local.spawnedRoom`))))
    (else
      (goto _label)))
  (return (`local.spawnedRoom`) (`local.failedToSpawn`)))

(fn `UserConstructionScript`)