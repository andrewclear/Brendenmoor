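; BP_Wolf is a wolf enemy Blueprint that decides whether the wolf is resting based on the time of day.
; Shortly after BeginPlay, a delayed call to UpdateRestingStatus reads the time from SkyBlueprintWrapper, if valid, and sets Resting for a window from midday to late evening.
; The check runs only once here, with no Tick or repeating update.
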(event `self.ReceiveBeginPlay`
  (`KismetSystemLibrary.Delay` 1.0)
  (`self.UpdateRestingStatus`))

(fn `UpdateRestingStatus`
  (bind _skyblueprintwrapper (`self.SkyBlueprintWrapper`))
  (if (`KismetSystemLibrary.IsValid` _skyblueprintwrapper)
    (bind _returnvalue (`SkyBlueprintWrapper.GetTimeOfDay` _skyblueprintwrapper))
    (set `self.Resting` (and (>= _returnvalue 12.0) (<= _returnvalue 22.0)))))

(fn `UserConstructionScript`)