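; Wrapper Blueprint around BP_FastStylizedProceduralSky that exposes the sky's time of day.
; On BeginPlay it casts SkyBlueprintReference to the sky class and caches it, printing an error message if the cast fails.
; GetTimeOfDay reads TimeOfDay from the cached sky when it is valid and returns it as Time.
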(event `self.ReceiveBeginPlay`
  (bind _asbp_fast_stylized_procedural_sky (cast `/Game/FastStylizedProceduralSky2/BP_FastStylizedProceduralSky` (`self.SkyBlueprintReference`))
    (:`then`
      (set `self.SkyBlueprint` _asbp_fast_stylized_procedural_sky))
    (:`CastFailed`
      (`KismetSystemLibrary.PrintString` "failed to cast sky reference to the sky blueprint" true true (struct :`G` 0.66 :`B` 1.0 :`A` 1.0) 5.0))))

(fn `GetTimeOfDay`
  (returns (ReturnValue :type "Float (double-precision)"))
  (locals (time :type "Float (double-precision)"))
  (bind _skyblueprint (`self.SkyBlueprint`))
  (if (`KismetSystemLibrary.IsValid` _skyblueprint)
    (set `local.time` (`/Game/FastStylizedProceduralSky2/BP_FastStylizedProceduralSky.TimeOfDay` _skyblueprint)))
  (return (`local.time`)))

(fn `UserConstructionScript`)